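; Player pawn for an Su-33 jet, flown with Enhanced Input thrust and roll plus mouse-position steering, starting with landing gear retracted.
; Tick smooths pitch and yaw from cursor offset via TurnMultipliers, banks the spring arm with yaw, and conditionally auto-levels roll, more slowly near vertical.
; Thrust feeds ACFlyingMovement, whose current value scales the animated exhaust nozzles and both Niagara jet effects.
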(event `EnhancedInput|/Game/Blueprints/Player/Input/IA_Thrust`
  (params (ActionValue :type "Float (double-precision)") (ElapsedSeconds :type "Float (double-precision)") (TriggeredSeconds :type "Float (double-precision)") (InputAction :type "InputAction Object Reference" :default "/Game/Blueprints/Player/Input/IA_Thrust.IA_Thrust"))
  (:`Triggered`
    (`/Game/Blueprints/FlyingMovement/AC_FlyingMovement.AddThrust` (`self.AC_FlyingMovement`) ActionValue)))

(event `self.ReceiveBeginPlay`
  (`EnhancedInputSubsystemInterface.AddMappingContext` (pcsubsystem `EnhancedInputLocalPlayerSubsystem` (cast `PlayerController` (`self.GetController`) :!pure true)) "/Game/Blueprints/Player/Input/IMP_Plane.IMP_Plane" 0 (struct))
  (bind _asbpa_east_fighter_su_33 (cast `/Game/VigilanteContent/Vehicles/East_Fighter_Su33/BPA_East_Fighter_Su33` (`SkeletalMeshComponent.GetAnimInstance` (`self.SkeletalMesh`))))
  (set `self.AnimInstance` _asbpa_east_fighter_su_33)
  (set `/Game/VigilanteContent/Vehicles/East_Fighter_Su33/BPA_East_Fighter_Su33.RearWheelRRetract` 1.0 (`self.AnimInstance`))
  (set `/Game/VigilanteContent/Vehicles/East_Fighter_Su33/BPA_East_Fighter_Su33.RearWheelLRetract` 1.0 (`self.AnimInstance`))
  (set `/Game/VigilanteContent/Vehicles/East_Fighter_Su33/BPA_East_Fighter_Su33.FrontWheelRetract` 1.0 (`self.AnimInstance`)))

(event `EnhancedInput|/Game/Blueprints/Player/Input/IA_Roll`
  (params (ActionValue :type "Float (double-precision)") (ElapsedSeconds :type "Float (double-precision)") (TriggeredSeconds :type "Float (double-precision)") (InputAction :type "InputAction Object Reference" :default "/Game/Blueprints/Player/Input/IA_Roll.IA_Roll"))
  (:`Triggered`
    (bind _output_get (set `self.X(Roll)` ActionValue :!label _label))
    (`self.K2_AddActorLocalRotation` (`KismetMathLibrary.MakeRotator` (* _output_get 180.0 (`GameplayStatics.GetWorldDeltaSeconds`)))))
  (:`Started`
    (goto _label))
  (:`Completed`
    (goto _label)))

(event `self.ReceiveTick`
  (params (DeltaSeconds :type "Float (single-precision)"))
  (bind _returnvalue_roll (`KismetMathLibrary.BreakRotator` (`self.K2_GetActorRotation`)))
  (bind _returnvalue_x (`KismetMathLibrary.BreakVector2D` (`/Game/Blueprints/GeneralFunctions.MousePositionFromOrigin`)))
  (bind _returnvalue (`GameplayStatics.GetWorldDeltaSeconds`))
  (bind _returnvalue_2 (`GameplayStatics.GetWorldDeltaSeconds`))
  (bind (_returnvalue_roll_2 _returnvalue_pitch) (`KismetMathLibrary.BreakRotator` (`self.K2_GetActorRotation`)))
  (bind (_returnvalue_roll_3 _returnvalue_pitch_2 _returnvalue_yaw) (`KismetMathLibrary.BreakRotator` (`self.K2_GetActorRotation`)))
  (bind (_z_yaw_ _y_pitch_) (`self.TurnMultipliers`))
  (bind _relativerotation_roll (`KismetMathLibrary.BreakRotator` (`SceneComponent.RelativeRotation` (`self.SpringArm1`))))
  (bind _returnvalue_3 (`KismetMathLibrary.MapRangeClamped` (`/Game/Blueprints/FlyingMovement/AC_FlyingMovement.CurrentThrust` (`self.AC_FlyingMovement`)) 0.0 2000.0 0.6 1.0))
  (bind _returnvalue_4 (* _returnvalue_3 11.5))
  (bind _returnvalue_5 (* _returnvalue_3 0.87))
  (bind _returnvalue_6 (* _returnvalue_5 0.375))
  (`|ExecutionSequence`
    (:`then_0`
      (set `self.Z(Yaw)` (`KismetMathLibrary.FInterpTo` (`self.Z(Yaw)`) _z_yaw_ _returnvalue_2 10.0))
      (set `self.Y(Pitch)` (`KismetMathLibrary.FInterpTo` (`self.Y(Pitch)`) _y_pitch_ _returnvalue_2 10.0))
      (`self.K2_AddActorLocalRotation` (`KismetMathLibrary.MakeRotator` 0.0 (* 60.0 (* (`self.Y(Pitch)`) -1.0) _returnvalue) (* 60.0 (`self.Z(Yaw)`) _returnvalue)))
      (`SceneComponent.K2_SetRelativeRotation` (`self.SpringArm1`) (`KismetMathLibrary.MakeRotator` (`KismetMathLibrary.FInterpTo_Constant` _relativerotation_roll (* (`self.Z(Yaw)`) 45.0) (`GameplayStatics.GetWorldDeltaSeconds`) 90.0)) false false)
      (if (and (== (`self.X(Roll)`) 0.0) (<= _returnvalue_x 100.0))
        (`self.K2_SetActorRotation` (`KismetMathLibrary.MakeRotator` (`KismetMathLibrary.FInterpTo_Constant` _returnvalue_roll 0.0 (`GameplayStatics.GetWorldDeltaSeconds`) (* (`KismetMathLibrary.MapRangeClamped` (/ (`KismetMathLibrary.Abs` _returnvalue_pitch) 90.0) 0.0 1.0 1.0) 60.0)) _returnvalue_pitch_2 _returnvalue_yaw))))
    (:`then_1`
      (set `/Game/VigilanteContent/Vehicles/East_Fighter_Su33/BPA_East_Fighter_Su33.ExhaustNozzles` _returnvalue_3 (`self.AnimInstance`))
      (`NiagaraComponent.SetVariableVec3` (`self.Niagara`) "JetRingsScale" (`KismetMathLibrary.MakeVector` _returnvalue_4 _returnvalue_4 (* _returnvalue_4 0.67)))
      (`NiagaraComponent.SetVariableVec3` (`self.Niagara1`) "JetRingsScale" (`KismetMathLibrary.MakeVector` _returnvalue_4 _returnvalue_4 (* _returnvalue_4 0.67)))
      (`NiagaraComponent.SetVariableVec3` (`self.Niagara`) "JetScale" (`KismetMathLibrary.MakeVector` _returnvalue_5 _returnvalue_6 _returnvalue_6))
      (`NiagaraComponent.SetVariableVec3` (`self.Niagara1`) "JetScale" (`KismetMathLibrary.MakeVector` _returnvalue_5 _returnvalue_6 _returnvalue_6))
      (`NiagaraComponent.SetVariableFloat` (`self.Niagara1`) "SpriteScale" _returnvalue_3)
      (`NiagaraComponent.SetVariableFloat` (`self.Niagara`) "SpriteScale" _returnvalue_3)
      (`NiagaraComponent.SetVariableFloat` (`self.Niagara`) "RingOpacity" (- _returnvalue_3 0.45))
      (`NiagaraComponent.SetVariableFloat` (`self.Niagara1`) "RingOpacity" (- _returnvalue_3 0.45)))))

(fn `UserConstructionScript`)