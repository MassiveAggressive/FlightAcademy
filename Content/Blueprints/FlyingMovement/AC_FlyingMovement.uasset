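; AC_FlyingMovement is an actor component that gives its owner simple thrust-driven forward flight.
; AddThrust accumulates a frame-time-scaled, clamped thrust value.
; Each tick, speed snaps up to that thrust, or eases down at a constant Drag rate when thrust is lower.
; The component then moves the owner along its local X axis by that speed, scaled by delta time.
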(event `self.ReceiveTick`
  (params (DeltaSeconds :type "Float (single-precision)"))
  (`self.CalculateSpeed`)
  (`self.UpdateOwnersPosition`))

(fn `AddThrust`
  (params (ThrustMultiplier :type "Float (double-precision)"))
  (set `self.CurrentThrust` (`KismetMathLibrary.FClamp` (+ (`self.CurrentThrust`) (* ThrustMultiplier (`self.Thrust`) (`GameplayStatics.GetWorldDeltaSeconds`))) 0.0 (`self.MaxThrust`))))

(fn `CalculateSpeed`
  (set `self.CurrentSpeed` (`KismetMathLibrary.SelectFloat` (`KismetMathLibrary.FInterpTo_Constant` (`self.CurrentSpeed`) (`self.CurrentThrust`) (`GameplayStatics.GetWorldDeltaSeconds`) (`self.Drag`)) (`self.CurrentThrust`) (< (`self.CurrentThrust`) (`self.CurrentSpeed`)))))

(fn `UpdateOwnersPosition`
  (`Actor.K2_AddActorLocalOffset` (`self.GetOwner`) (`KismetMathLibrary.MakeVector` (* (`self.CurrentSpeed`) (`GameplayStatics.GetWorldDeltaSeconds`))) false false))